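; GA_Flash is a player gameplay ability that performs a forward flash (dash) movement.
; On activation it commits, disables movement on the first player controller, and runs an ATMove task along the avatar's forward vector for a fixed distance and speed.
; When the move ends, it re-enables movement and ends the ability; the OnEndAbility event is empty, so movement is restored only on that callback.
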(event `self.K2_ActivateAbility`
  (`self.K2_CommitAbility`)
  (bind _asrlplayer_controller (cast `RLPlayerController` (`GameplayStatics.GetPlayerController` 0)))
  (`RLPlayerController.SetCanMove` _asrlplayer_controller false)
  (`AT_Move.CreateATMove` (`Actor.GetActorForwardVector` (`self.GetAvatarActorFromActorInfo`)) 500.0 100.0
    (:`OnMoveEnd`
      (bind _asrlplayer_controller_2 (cast `RLPlayerController` (`GameplayStatics.GetPlayerController` 0)))
      (`RLPlayerController.SetCanMove` _asrlplayer_controller_2 true)
      (`self.K2_EndAbility`))))