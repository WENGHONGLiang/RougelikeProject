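; Player gameplay ability that dashes the avatar forward while knocking back and damaging nearby enemies.
; On activation it commits, disables movement on the RL player controller and runs an ATMove task along the actor's forward vector.
; The task's looping event periodically calls BeatBackEnemyAroundPlayer to push surrounding enemies with impulse and damage.
; When the move ends, the ability ends and movement is re-enabled.
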(event `self.K2_ActivateAbility`
  (`self.K2_CommitAbility`)
  (bind _asrlplayer_controller (cast `RLPlayerController` (`GameplayStatics.GetPlayerController` 0)))
  (`RLPlayerController.SetCanMove` _asrlplayer_controller false)
  (`AT_Move.CreateATMove` (`Actor.GetActorForwardVector` (`self.GetAvatarActorFromActorInfo`)) 1000.0 1.0 true 0.5
    (:`OnMoveEnd`
      (`self.K2_EndAbility`)
      (bind _asrlplayer_controller_2 (cast `RLPlayerController` (`GameplayStatics.GetPlayerController` 0)))
      (`RLPlayerController.SetCanMove` _asrlplayer_controller_2 true))
    (:`OnLoopEvent`
      (`self.BeatBackEnemyAroundPlayer` 200.0 700.0 true))))