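; Player gameplay ability that fires a projectile while moving the avatar backward, opposite its facing.
; On activation it commits, stores the cursor hit as the target location, or ends if nothing is hit, and disables player movement.
; A custom ATMove task drives the retreat alongside the attack montage, whose gameplay event triggers the projectile spawn.
; Move completion, rather than montage completion, restores movement and ends the ability.
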(event `self.K2_ActivateAbility`
  (bind (_bblockinghit _binitialoverlap _time _distance _location) (`GameplayStatics.BreakHitResult` (`PlayerController.GetHitResultUnderCursorByChannel` (`GameplayStatics.GetPlayerController` 0) "TraceTypeQuery1" true)))
  (`self.K2_CommitAbility`)
  (if _bblockinghit
    (set `self.TargetLocation` _location)
    (bind _asrlplayer_controller (cast `RLPlayerController` (`GameplayStatics.GetPlayerController` 0)))
    (`RLPlayerController.SetCanMove` _asrlplayer_controller false)
    (`AT_Move.CreateATMove` (- (0.0 0.0 0.0) (`Actor.GetActorForwardVector` (`self.GetAvatarActorFromActorInfo`))) 300.0 5.0
      (:`then`
        (`AbilityTask_PlayMontageAndWait.CreatePlayMontageAndWaitProxy` "None" (`RLCharacterBase.AttackAnim` (`self.GetCharacterBase`))
          (:`then`
            (`AbilityTask_WaitGameplayEvent.WaitGameplayEvent` (struct :`TagName` "Event.Montage.Projectile") null
              (:`EventReceived`
                (`self.SpawnProjectile`))))))
      (:`OnMoveEnd`
        (bind _asrlplayer_controller_2 (cast `RLPlayerController` (`GameplayStatics.GetPlayerController` 0)))
        (`RLPlayerController.SetCanMove` _asrlplayer_controller_2 true)
        (`self.K2_EndAbility`)))
    (else
      (`self.K2_EndAbility`))))