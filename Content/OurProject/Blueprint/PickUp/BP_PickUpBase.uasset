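; Base pickup actor that shows a HUD tip on overlap and destroys itself when the player picks it up.
; Any begin overlap sets a collision flag, calls TipCall on BP_Hero's MainUI, stores the result, and binds the PickUp event to the hero.
; PickUp destroys the actor only while the flag is set.
; End overlap clears the flag and removes MainUI itself from its parent, leaving the binding in place.
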(event `self.ReceiveActorBeginOverlap`
  (params (OtherActor :type "Actor Object Reference"))
  ;[1 1 1] 发生碰撞后，获取玩家（BP_Hero）身上的MainUI变量，调用WBP_HUD里的函数(tipCall)创建Pickup
  (set `self.isCollision` true)
  (bind _asbp_hero (cast `/Game/OurProject/Blueprint/BP_Character/BP_Hero` (`GameplayStatics.GetPlayerPawn` 0)))
  (bind _returnvalue (`/Game/OurProject/Blueprint/UI/WBP_HUD.TipCall` (`/Game/OurProject/Blueprint/BP_Character/BP_Hero.MainUI` _asbp_hero)))
  (set `self.TIp` _returnvalue)
  (add `/Game/OurProject/Blueprint/BP_Character/BP_Hero.PickUp` _asbp_hero (delegate `PickUp`)))

(event `PickUp`
  (if (`self.isCollision`)
    (`self.K2_DestroyActor`)))

(event `self.ReceiveActorEndOverlap`
  (params (OtherActor :type "Actor Object Reference"))
  (set `self.isCollision` false)
  (bind _asbp_hero (cast `/Game/OurProject/Blueprint/BP_Character/BP_Hero` (`GameplayStatics.GetPlayerPawn` 0)))
  (`Widget.RemoveFromParent` (`/Game/OurProject/Blueprint/BP_Character/BP_Hero.MainUI` _asbp_hero)))

(fn `UserConstructionScript`)