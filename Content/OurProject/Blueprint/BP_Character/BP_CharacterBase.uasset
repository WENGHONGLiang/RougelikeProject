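; BP_CharacterBase is a character Blueprint that exercises its AC_ChaHealth health component through debug key bindings.
; The 0 key calls Hurt and the 2 key calls Healing, each with a fixed amount.
; The component's hurt, healing and death events each print a debug string, with no other gameplay response.
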(event `Key|Zero`
  (params (Key :type "Key Structure"))
  (:`Pressed`
    (`/Game/OurProject/Blueprint/BP_Character/AC_ChaHealth.Hurt` (`self.AC_ChaHealth`) 50.0)))

(event `Key|Two`
  (params (Key :type "Key Structure"))
  (:`Pressed`
    (`/Game/OurProject/Blueprint/BP_Character/AC_ChaHealth.Healing` (`self.AC_ChaHealth`) 50.0)))

(event `self.AC_ChaHealth.OnHurt`
  (`KismetSystemLibrary.PrintString` "getHurt"))

(event `self.AC_ChaHealth.OnHealing`
  (`KismetSystemLibrary.PrintString` "getHeal"))

(event `self.AC_ChaHealth.OnDeath`
  (`KismetSystemLibrary.PrintString` "I'm dead"))

(fn `UserConstructionScript`)