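; Actor component that tracks health for its owning actor, presumably a character, starting at full HP on BeginPlay.
; Hurt and Healing clamp HP between zero and max, ignore calls once dead, and fire hurt, healing, death and health-changed dispatchers.
; Death and Alive are queries derived from current HP.
; A max-HP setter scales current HP by a max-HP ratio, apparently to preserve the health percentage.
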(event `self.ReceiveBeginPlay`
  (set `self.CurrentHp` (`self.MaxHp`))
  (`self.OnHealthChanged`))

(fn `Alive`
  (returns (ReturnValue :type Boolean))
  (return (not (`self.Death`))))

(fn `Death`
  (returns (ReturnValue :type Boolean))
  (return (<= (`self.CurrentHp`) 0.0)))

(fn `Healing`
  (params (HealingNum :type "Float (double-precision)"))
  (if (not (`self.Death`))
    (set `self.CurrentHp` (`KismetMathLibrary.FMin` (+ (`self.CurrentHp`) HealingNum) (`self.MaxHp`)))
    (`self.OnHealing`)
    (`self.OnHealthChanged`)))

(fn `Hurt`
  (params (Damage :type "Float (double-precision)"))
  (if (`self.Alive`)
    (bind _output_get (set `self.CurrentHp` (`KismetMathLibrary.FMax` (- (`self.CurrentHp`) Damage))))
    (`self.OnHurt`)
    (`self.OnHealthChanged`)
    (if (<= _output_get 0.0)
      (`self.OnDeath`))))

(fn `SetMaxHp_CurrentHp`
  (params (MaxHp :type "Float (double-precision)"))
  (locals (Scale :type "Float (double-precision)"))
  (set `local.Scale` (/ MaxHp (`self.MaxHp`)))
  (set `self.MaxHp` MaxHp)
  (set `self.CurrentHp` (* (`self.CurrentHp`) (`local.Scale`)))
  (`self.OnHealthChanged`))