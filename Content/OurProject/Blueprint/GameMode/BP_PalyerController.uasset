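; Player controller whose only working logic opens the pause menu.
; Pressing Tab creates a WBP_Pause widget, adds it to the viewport, switches input to UI only and shows the mouse cursor, without itself pausing the game.
; Nodes for adding the Enhanced Input mapping context, moving the pawn and starting or stopping BP_Hero fire are disconnected and never run.
; BeginPlay, Tick and the IA_Move event are empty.
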(event `EnhancedInput|/Game/OurProject/Input/Actions/IA_Move`
  (params (ActionValue :type "Vector2D Structure") (ElapsedSeconds :type "Float (double-precision)") (TriggeredSeconds :type "Float (double-precision)") (InputAction :type "InputAction Object Reference" :default "/Game/OurProject/Input/Actions/IA_Move.IA_Move")))

(event `self.ReceiveBeginPlay`)

(event `EnhancedInput|/Game/OurProject/Input/Actions/IA_Fire`
  (params (ActionValue :type Boolean) (ElapsedSeconds :type "Float (double-precision)") (TriggeredSeconds :type "Float (double-precision)") (InputAction :type "InputAction Object Reference" :default "/Game/OurProject/Input/Actions/IA_Fire.IA_Fire"))
  ;[1 1 1] 鼠标左键控制玩家身上的开火和停火方法
)

(event `Key|Tab`
  (params (Key :type "Key Structure"))
  ;[1 1 1] TAB键控制暂停界面
  (:`Pressed`
    (bind _returnvalue (`|CreateWidget` "/Game/OurProject/Blueprint/UI/WBP_Pause.WBP_Pause_C"))
    (`UserWidget.AddToViewport` _returnvalue 0)
    (`WidgetBlueprintLibrary.SetInputMode_UIOnlyEx` self null)
    (set `self.bShowMouseCursor` true)))

(fn `UserConstructionScript`)