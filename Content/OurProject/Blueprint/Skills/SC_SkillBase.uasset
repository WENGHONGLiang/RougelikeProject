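; SC_SkillBase is a base Blueprint for skills that fire while a firing flag is on.
; OpenFire and StopFire toggle IsFire, and Tick counts RemainTime down, calling the empty Fire event when time runs out and the flag is set.
; After firing, CDTime is assigned to itself and RemainTime is not reset, so Fire repeats every tick while the flag stays on.
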(event `self.ReceiveTick`
  (params (DeltaSeconds :type "Float (single-precision)"))
  (set `self.RemainTime` (- (`self.RemainTime`) DeltaSeconds))
  (if (<= (`self.RemainTime`) 0.0)
    (if (`self.isFire`)
      (`self.Fire`)
      (set `self.CDTime` (`self.CDTime`)))))

(event `Fire`)

(fn `OpenFire`
  (set `self.isFire` true))

(fn `StopFire`
  (set `self.isFire` false))